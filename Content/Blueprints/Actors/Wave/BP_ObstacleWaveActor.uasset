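; Wave obstacle actor that damages player characters when they overlap its Box component.
; On the server, the begin-overlap event casts to MSPlayerCharacter and applies the BPGE_ObstacleCollisionDamage Gameplay Effect to that character's Ability System Component.
; Damage is applied once per overlap, as the looping timer for repeat damage is disconnected and both DamageEvent and the end-overlap handler are empty.
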(event OnComponentBeginOverlap(Box)
  (params (OverlappedComponent :type Primitive%20Component%20Object%20Reference) (OtherActor :type Actor%20Object%20Reference) (OtherComp :type Primitive%20Component%20Object%20Reference) (OtherBodyIndex :type Integer) (bFromSweep :type Boolean) (SweepResult :type Hit%20Result%20Structure%20%28by%20ref%29))
  (if (Ability|HasAuthority)
    (bind _asmsplayer_character (Utilities|Casting|CastToMSPlayerCharacter OtherActor))
    (Variables|Default|SetASC (Ability|GetAbilitySystemComponent _asmsplayer_character))
    (GameplayEffects|ApplyGameplayEffectSpecToSelf (Ability|GetAbilitySystemComponent _asmsplayer_character) (GameplayEffects|MakeOutgoingSpec (Ability|GetAbilitySystemComponent _asmsplayer_character) "/Game/Blueprints/GAS/GE/BPGE_ObstacleCollisionDamage.BPGE_ObstacleCollisionDamage_C" 0.0 (GameplayEffects|MakeEffectContext (Ability|GetAbilitySystemComponent _asmsplayer_character))))))

(event OnComponentEndOverlap(Box)
  (params (OverlappedComponent :type Primitive%20Component%20Object%20Reference) (OtherActor :type Actor%20Object%20Reference) (OtherComp :type Primitive%20Component%20Object%20Reference) (OtherBodyIndex :type Integer)))

(event Custom|DamageEvent)

(event EventBeginPlay)

(event Collision|EventActorBeginOverlap
  (params (OtherActor :type Actor%20Object%20Reference)))

(event EventTick
  (params (DeltaSeconds :type Float%20%28single-precision%29)))

(fn ConstructionScript)